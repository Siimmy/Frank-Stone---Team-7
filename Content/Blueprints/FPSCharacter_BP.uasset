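; Player character Blueprint with Enhanced Input movement, switchable first/third-person cameras, an inventory screen and a game-over screen.
; A capsule trace from the third-person camera, regardless of active view, drives interface-based interaction and the per-tick crosshair update.
; The spawned flashlight drains battery on a looping timer feeding the HUD, with inventory batteries restoring charge.
; A flashlight collision overlap makes enemy AI run away and is disabled when the battery empties.
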(event `self.ReceiveBeginPlay`
  ;[1 1 1] Add input controls - add widget crosshair and battery power
  (bind _asplayer_controller (cast `PlayerController` (`self.GetController`)))
  (bind _returnvalue (pcsubsystem `EnhancedInputLocalPlayerSubsystem` _asplayer_controller))
  (`/Engine/EditorBlueprintResources/StandardMacros.IsValid` _returnvalue
    (:`Is Valid`
      (`EnhancedInputSubsystemInterface.AddMappingContext` _returnvalue "/Game/Input/FPS_IMC.FPS_IMC" 0 (struct))
      (bind _returnvalue_2 (`|CreateWidget` "/Game/UserInterfaces/Player_WB.Player_WB_C" null null))
      (bind _output_get (set `self.PlayerHUD` _returnvalue_2))
      (`UserWidget.AddToViewport` _output_get 0)
      ;[1 1 1] Start with torch?
      (set `self.Hasflightlight?` true)
      (`self.Toggle flashlight`))))

(event `EnhancedInput|/Game/Input/Move_IA`
  (params (ActionValue :type "Vector2D Structure") (ElapsedSeconds :type "Float (double-precision)") (TriggeredSeconds :type "Float (double-precision)") (InputAction :type "InputAction Object Reference" :default "/Game/Input/Move_IA.Move_IA"))
  ;[1 1 1] Handle movement
  (:`Triggered`
    (`self.AddMovementInput` (`self.GetActorRightVector`) ActionValue_X)
    (`self.AddMovementInput` (`self.GetActorForwardVector`) ActionValue_Y)
    (if (> (`KismetMathLibrary.VSize` (`self.GetVelocity`)) 0.0)
      _)))

(event `EnhancedInput|/Game/Input/Look_IA`
  (params (ActionValue :type "Vector2D Structure") (ElapsedSeconds :type "Float (double-precision)") (TriggeredSeconds :type "Float (double-precision)") (InputAction :type "InputAction Object Reference" :default "/Game/Input/Look_IA.Look_IA"))
  ;[1 1 1] Handle camera movement
  (:`Triggered`
    (`self.AddControllerYawInput` ActionValue_X)
    (`self.AddControllerPitchInput` ActionValue_Y)))

(event `EnhancedInput|/Game/Input/Jump_IA`
  (params (ActionValue :type Boolean) (ElapsedSeconds :type "Float (double-precision)") (TriggeredSeconds :type "Float (double-precision)") (InputAction :type "InputAction Object Reference" :default "/Game/Input/Jump_IA.Jump_IA"))
  ;[1 1 1] Handle jumping
  (:`Started`
    (`self.Jump`))
  (:`Canceled`
    (`self.StopJumping`)))

(event `Close inventory`
  (bind _returnvalue (`GameplayStatics.GetPlayerController` 0))
  ;[1 1 1] Toggle inventory
  (`/Engine/EditorBlueprintResources/StandardMacros.IsValid` (`self.Inventoryhud`)
    (:`Is Valid`
      (`Widget.RemoveFromParent` (`self.Inventoryhud`))
      (set `PlayerController.bShowMouseCursor` false _returnvalue)
      (`WidgetBlueprintLibrary.SetInputMode_GameOnly` _returnvalue)
      (set `self.Inventoryhud` null)
      (`self.EnableInput` self _returnvalue))))

(event `EnhancedInput|/Game/Input/Inventory_IA`
  (params (ActionValue :type Boolean) (ElapsedSeconds :type "Float (double-precision)") (TriggeredSeconds :type "Float (double-precision)") (InputAction :type "InputAction Object Reference" :default "/Game/Input/Inventory_IA.Inventory_IA"))
  (bind _returnvalue (`GameplayStatics.GetPlayerController` 0))
  (bind _inventoryhud (`self.Inventoryhud`))
  ;[1 1 1] Toggle inventory
  (:`Started`
    (`self.Inventoryhud`
      (:`then`)
      (:`else`
        (bind _returnvalue_2 (`|CreateWidget` "/Game/UserInterfaces/Inventory_WB.Inventory_WB_C" null null))
        (set `self.Inventoryhud` _returnvalue_2)
        (for _array_element (`self.Inventory`)
          (`/Game/UserInterfaces/Inventory_WB.Add inventory items` _inventoryhud _array_element))
        (`UserWidget.AddToViewport` _inventoryhud 0)
        (set `PlayerController.bShowMouseCursor` true _returnvalue)
        (`WidgetBlueprintLibrary.SetInputMode_GameAndUIEx` _returnvalue null)
        (`self.DisableInput` self _returnvalue)))))

(event `EnhancedInput|/Game/Input/Interact_IA`
  (params (ActionValue :type Boolean) (ElapsedSeconds :type "Float (double-precision)") (TriggeredSeconds :type "Float (double-precision)") (InputAction :type "InputAction Object Reference" :default "/Game/Input/Interact_IA.Interact_IA"))
  (bind _thirdpersoncamera (`self.ThirdPersonCamera`))
  (bind _returnvalue (`SceneComponent.K2_GetComponentLocation` _thirdpersoncamera))
  ;[1 1 1] Handle interaction - THIRD PERSON CAMERA
  (:`Triggered`
    (bind _outhit (`KismetSystemLibrary.CapsuleTraceSingle` _returnvalue (+ _returnvalue (* (`KismetMathLibrary.GetForwardVector` (`SceneComponent.K2_GetComponentRotation` _thirdpersoncamera)) (`self.Interactdistance`))) 17.0 17.0 "TraceTypeQuery1"))
    (bind (_bblockinghit _binitialoverlap _time _distance _location _impactpoint _normal _impactnormal _physmat _hitactor) (`GameplayStatics.BreakHitResult` _outhit))
    (if (`KismetSystemLibrary.DoesImplementInterface` _hitactor "/Game/Blueprints/Interactinterface.Interactinterface_C")
      (message `/Game/Blueprints/Interactinterface.Interact` _hitactor self))))

(event `Toggle flashlight`
  ;[1 1 1] Handle flashlight
  (if (`self.Hasflightlight?`) :!label _label
    (`/Engine/EditorBlueprintResources/StandardMacros.IsValid` (`self.flashlighref`)
      (:`Is Valid`
        (`GameplayStatics.PlaySoundAtLocation` "/Game/SFX/ButtonOn01.ButtonOn01" (`self.K2_GetActorLocation`) (struct) 1.0 1.0 0.0 null null null null)
        (`self.K2_DestroyActor` (`self.flashlighref`))
        (set `self.flashlighref` null)
        (`Widget.SetVisibility` (`/Game/UserInterfaces/Player_WB.flashlightbox` (`self.PlayerHUD`)) "Hidden")
        (`KismetSystemLibrary.K2_ClearAndInvalidateTimerHandle` (`self.drainflashlight`)))
      (:`Is Not Valid`
        (`GameplayStatics.PlaySoundAtLocation` "/Game/SFX/ButtonOn01.ButtonOn01" (`self.K2_GetActorLocation`) (struct) 1.0 1.0 0.0 null null null null)
        (bind _returnvalue (`|SpawnActorFromClass` "/Game/Blueprints/Flashlight_BP.Flashlight_BP_C" (`SceneComponent.K2_GetComponentToWorld` (`self.Flashlight`)) "Undefined" "MultiplyWithRoot" null null))
        (bind _output_get (set `self.flashlighref` _returnvalue))
        (`self.K2_AttachToComponent` _output_get (`self.Flashlight`) "None" "SnapToTarget" "SnapToTarget" "SnapToTarget" true)
        ;;[1 1 1] Show flashlight bar
        (`Widget.SetVisibility` (`/Game/UserInterfaces/Player_WB.flashlightbox` (`self.PlayerHUD`)) "Visible")
        (bind _returnvalue_2 (`KismetSystemLibrary.K2_SetTimerDelegate` (delegate `DrainBattery`) 0.001 true))
        (set `self.drainflashlight` _returnvalue_2)))))

(event `DrainBattery`
  (bind _flashlighref (`self.flashlighref`))
  ;[1 1 1] Handle flashlight
  (bind _output_get (set `self.battery` (- (`self.battery`) (`self.batterydrainrate`))))
  (`/Game/UserInterfaces/Player_WB.Update battery` (`self.PlayerHUD`) _output_get)
  ;;[1 1 1] If <= o turn off flashlight
  (if (<= _output_get 0.0)
    (`/Engine/EditorBlueprintResources/StandardMacros.IsValid` _flashlighref
      (:`Is Valid`
        (`/Game/Blueprints/Flashlight_BP.Turn off flashlight` _flashlighref)
        (`KismetSystemLibrary.K2_ClearAndInvalidateTimerHandle` (`self.drainflashlight`))
        (`/Game/UserInterfaces/Player_WB.Update battery` (`self.PlayerHUD`) _output_get)
        ;;[1 1 1] Disable collision if battery == 0
        (`PrimitiveComponent.SetCollisionEnabled` (`self.FlashCollision`) "NoCollision")))))

(event `EnhancedInput|/Game/Input/Flashlight_IA`
  (params (ActionValue :type Boolean) (ElapsedSeconds :type "Float (double-precision)") (TriggeredSeconds :type "Float (double-precision)") (InputAction :type "InputAction Object Reference" :default "/Game/Input/Flashlight_IA.Flashlight_IA"))
  ;[1 1 1] Handle flashlight
  (:`Started`
    (goto _label)))

(event `TransitionCameraToFirstPerson`
  ;[1 1 1] Transition Camera - NOT IN USE - testing only
  (set `CameraComponent.bUsePawnControlRotation` false (`self.ThirdPersonCamera`))
  (bind (_direction _transitionoutput) (`Timeline|Timeline` :!via `PlayFromStart`)
    (:`Update`
      (`SceneComponent.K2_SetWorldTransform` (`self.ThirdPersonCamera`) (`KismetMathLibrary.TLerp` (`SceneComponent.K2_GetComponentToWorld` (`self.ThirdPersonCamera`)) (`SceneComponent.K2_GetComponentToWorld` (`self.Camera`)) _transitionoutput) false false)
      (`KismetSystemLibrary.Delay` 3.0)
      (bind (_direction_2 _transitionoutput_2) (`Timeline|TransitionBack` :!via `PlayFromStart`)
        (:`Update`
          (`SceneComponent.K2_SetWorldTransform` (`self.ThirdPersonCamera`) (`KismetMathLibrary.TLerp` (`SceneComponent.K2_GetComponentToWorld` (`self.Camera`)) (`SceneComponent.K2_GetComponentToWorld` (`self.ThirdPersonCamera`)) _transitionoutput_2) false false))
        (:`Finished`
          (set `CameraComponent.bUsePawnControlRotation` true (`self.ThirdPersonCamera`)))))))

(event `Use battery`
  (bind _inventory (`self.Inventory`))
  (bind _inventory_2 (`self.Inventory`))
  (bind _flashlighref (`self.flashlighref`))
  ;[1 1 1] Use battery
  (for (_array_element _array_index) (`self.Inventory`)
    (if (== (`.Item_10_5B585F634281B3AECF1787A89A286F8B` (break `/Game/Blueprints/Inspection/ItemInformation` _array_element)) "/Game/Blueprints/Inspection/Batteryinv_bp.Batteryinv_bp_C")
      (`KismetArrayLibrary.Array_Set` _inventory _array_index)
      (if (> (`.Number_23_3B51E2014C6A05B3A09AB389937A2F3D` (break `/Game/Blueprints/Inspection/ItemInformation` _array_element)) 1)
        (`KismetArrayLibrary.Array_Set` _inventory _array_index (make `/Game/Blueprints/Inspection/ItemInformation` (break `/Game/Blueprints/Inspection/ItemInformation` _array_element) (`.ItemDescription_4_310DA46947E17BBAB126E68A97557B58` (break `/Game/Blueprints/Inspection/ItemInformation` _array_element)) (`.Itemimage_7_3D8D4B0040A2B8DE268A7FB5B6CB1E41` (break `/Game/Blueprints/Inspection/ItemInformation` _array_element)) (`.Item_10_5B585F634281B3AECF1787A89A286F8B` (break `/Game/Blueprints/Inspection/ItemInformation` _array_element)) (`.isstackable?_20_3124AB364B21F1FF48C6B1814701FF6B` (break `/Game/Blueprints/Inspection/ItemInformation` _array_element)) (- (`.Number_23_3B51E2014C6A05B3A09AB389937A2F3D` (break `/Game/Blueprints/Inspection/ItemInformation` _array_element)) 1)))
        (else
          (set `self.battery` 1.0)
          (`KismetArrayLibrary.Array_RemoveItem` _inventory_2 (`|GetArrayItem` _inventory_2 _array_index))))
      (bind _output_get (set `self.battery` 1.0))
      ;;[1 1 1] restart timer if at 0 and turn flashlight back on
      (`/Engine/EditorBlueprintResources/StandardMacros.IsValid` _flashlighref
        (:`Is Valid`
          (`/Game/Blueprints/Flashlight_BP.Turn on flashlight` _flashlighref)
          (`/Game/UserInterfaces/Player_WB.Update battery` (`self.PlayerHUD`) _output_get)
          (`KismetSystemLibrary.K2_SetTimerDelegate` (delegate `DrainBattery`) 0.001 true)
          ;;[1 1 1] Enable collision
          (`PrimitiveComponent.SetCollisionEnabled` (`self.FlashCollision`) "QueryOnly"))))))

(event `Key|N`
  (params (Key :type "Key Structure"))
  ;[1 1 1] Transition Camera - NOT IN USE - testing only
  (:`Pressed`
    (`self.TransitionCameraToFirstPerson`)))

(event `CollectedBattery`
  ;[1 1 1] Use battery
)

(event `ToggleCamera`
  ;[1 1 1] Transition Camera - NOT IN USE - testing only
  (if (`self.bIsInFirstPerson`)
    (`ActorComponent.SetActive` (`self.ThirdPersonCamera`) true false)
    (`ActorComponent.SetActive` (`self.Camera`) false false)
    (set `self.bIsInFirstPerson` false)
    (else
      (`ActorComponent.SetActive` (`self.Camera`) true false)
      (`ActorComponent.SetActive` (`self.ThirdPersonCamera`) false false)
      (set `self.bIsInFirstPerson` true))))

(event `self.FlashCollision.OnComponentBeginOverlap`
  (params (OverlappedComponent :type "PrimitiveComponent Object Reference") (OtherActor :type "Actor Object Reference") (OtherComp :type "PrimitiveComponent Object Reference") (OtherBodyIndex :type Integer) (bFromSweep :type Boolean) (SweepResult :type "HitResult Structure (by ref)"))
  ;[1 1 1] Flashlight collision - run away event called from enemy ai
  (bind _asai_enemy_bp (cast `/Game/Enemy/Blueprints/AI_ToUse/AI_Enemy_BP` OtherActor))
  (`/Game/Enemy/Blueprints/AI_ToUse/AI_Enemy_BP.RunAway` _asai_enemy_bp))

(event `self.ReceiveTick`
  (params (DeltaSeconds :type "Float (single-precision)"))
  ;[1 1 1] Update cross hair
  (`self.Updatecrosshair`))

(event `Key|V`
  (params (Key :type "Key Structure"))
  ;[1 1 1] Transition Camera - NOT IN USE - testing only
  (:`Pressed`
    (`self.ToggleCamera`)))

(event `self.FlashCollision.OnComponentEndOverlap`
  (params (OverlappedComponent :type "PrimitiveComponent Object Reference") (OtherActor :type "Actor Object Reference") (OtherComp :type "PrimitiveComponent Object Reference") (OtherBodyIndex :type Integer))
  ;[1 1 1] Flashlight collision - run away event called from enemy ai
  (bind _asai_enemy_bp (cast `/Game/Enemy/Blueprints/AI_ToUse/AI_Enemy_BP` OtherActor))
  (set `/Game/Enemy/Blueprints/AI_ToUse/AI_Enemy_BP.isChasing?` false _asai_enemy_bp)
  (`MovementComponent.StopMovementImmediately` (`self.CharacterMovement`)))

(event `Lose`
  ;[1 1 1] Lose event triggers lose screen and disables movement
  (bind _returnvalue (`|CreateWidget` "/Game/UserInterfaces/Gameover_WB.Gameover_WB_C"))
  (`UserWidget.AddToViewport` _returnvalue 0)
  (`CharacterMovementComponent.DisableMovement` (`self.CharacterMovement`)))

(fn `Updatecrosshair`
  (bind _thirdpersoncamera (`self.ThirdPersonCamera`))
  (bind _returnvalue (`SceneComponent.K2_GetComponentLocation` _thirdpersoncamera))
  (bind _outhit (`KismetSystemLibrary.CapsuleTraceSingle` _returnvalue (+ _returnvalue (* (`KismetMathLibrary.GetForwardVector` (`SceneComponent.K2_GetComponentRotation` _thirdpersoncamera)) (`self.Interactdistance`))) 17.0 17.0 "TraceTypeQuery1"))
  (if (`KismetSystemLibrary.DoesImplementInterface` (`.HitActor` (`GameplayStatics.BreakHitResult` _outhit)) "/Game/Blueprints/Interactinterface.Interactinterface_C")
    (`Image.SetBrushFromTexture` (`/Game/UserInterfaces/Player_WB.crosshair` (`self.PlayerHUD`)) "/Game/Images/crosshair003.crosshair003" false)
    (else
      (`Image.SetBrushFromTexture` (`/Game/UserInterfaces/Player_WB.crosshair` (`self.PlayerHUD`)) "/Game/Images/crosshair001.crosshair001" false))))

(fn `UserConstructionScript`)