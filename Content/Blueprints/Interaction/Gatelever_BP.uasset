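; Gatelever_BP is an interactable lever that signals other objects through a Triggerlever event dispatcher, presumably to operate a gate.
; When Activated, Interact plays a metal creak, broadcasts the dispatcher and uses a FlipFlop to alternately play or reverse a timeline.
; The timeline drives the lever's roll, and a DoOnce blocks repeat use until the swing finishes.
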(event `self.Interact`
  (params (fpscharacter :type "/Game/Blueprints/FPSCharacter_BP Object Reference"))
  (if (`self.Activated?`)
    (`/Engine/EditorBlueprintResources/StandardMacros.DoOnce` false :!label _label
      (:`Completed`
        (`GameplayStatics.PlaySoundAtLocation` "/Game/SFX/MetalCreak01.MetalCreak01" (`self.K2_GetActorLocation`) (struct) 1.0 1.0 0.0 null null null null)
        (`self.triggerlever`)
        (`/Engine/EditorBlueprintResources/StandardMacros.FlipFlop`
          (:`A`
            (bind (_direction _levertrack) (`Timeline|levertimeline` :!via `PlayFromStart` :!label _label_2)
              (:`Update`
                (`SceneComponent.K2_SetRelativeRotation` (`self.Lever`) (`KismetMathLibrary.MakeRotator` (`KismetMathLibrary.Lerp` 0.0 -30.0 _levertrack)) false false))
              (:`Finished`
                (goto _label :!via `Reset`))))
          (:`B`
            (goto _label_2 :!via `ReverseFromEnd`)))))))

(fn `UserConstructionScript`)