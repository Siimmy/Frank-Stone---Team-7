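; Base actor for inspectable items, examined from the world or opened from the player's inventory.
; Inspection moves input from the character to the item, attaches it before the camera, shows an Item_WB widget and rotates it with left-drag.
; Right-click collects world items, stacking inventory entries, with special handling for the flashlight and colored batteries.
; Inventory-opened items can be used via UseitemF or closed, both destroying the actor.
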(event `EnhancedInput|/Game/Input/Useitem_IA`
  (params (ActionValue :type Boolean) (ElapsedSeconds :type "Float (double-precision)") (TriggeredSeconds :type "Float (double-precision)") (InputAction :type "InputAction Object Reference" :default "/Game/Input/Useitem_IA.Useitem_IA"))
  ;[1 1 1] Z to remove Item
  (:`Started`
    (if (`self.FromInventory`)
      (`self.StopInspecting item`)
      (`/Game/Blueprints/FPSCharacter_BP.Close inventory` (`self.Fpscharacter`))
      (`/Game/Blueprints/Interactinterface.useitem_f`)
      ;;[1 1 1] Comment
      (`self.K2_DestroyActor`))))

(event `EnhancedInput|/Game/Input/Inventory_IA`
  (params (ActionValue :type Boolean) (ElapsedSeconds :type "Float (double-precision)") (TriggeredSeconds :type "Float (double-precision)") (InputAction :type "InputAction Object Reference" :default "/Game/Input/Inventory_IA.Inventory_IA"))
  ;[1 1 1] Q to look at inventory
  (:`Started`
    (if (`self.FromInventory`)
      (`self.StopInspecting item`)
      (`/Game/Blueprints/FPSCharacter_BP.Close inventory` (`self.Fpscharacter`))
      (`self.K2_DestroyActor`))))

(event `EnhancedInput|/Game/Input/Interact_IA`
  (params (ActionValue :type Boolean) (ElapsedSeconds :type "Float (double-precision)") (TriggeredSeconds :type "Float (double-precision)") (InputAction :type "InputAction Object Reference" :default "/Game/Input/Interact_IA.Interact_IA"))
  ;[1 1 1] E to Interact
  (:`Started`
    (if (not (`self.FromInventory`))
      (`self.StopInspecting item`))))

(event `Closeitem`
  ;[1 1 1] Close
  (`self.StopInspecting item`)
  (`self.K2_DestroyActor`))

(event `Open item from Inventory`
  ;[1 1 1] Comment
  (bind _asfpscharacter_bp (cast `/Game/Blueprints/FPSCharacter_BP` (`GameplayStatics.GetPlayerCharacter` 0)))
  (bind _output_get (set `self.Fpscharacter` _asfpscharacter_bp))
  (`/Game/Blueprints/FPSCharacter_BP.Inspecteditem` _output_get
    (:`then`)
    (:`else`
      (`self.Inspectitem`))))

(event `/Game/Blueprints/Interactinterface.Interact`
  (params (fpscharacter :type "/Game/Blueprints/FPSCharacter_BP Object Reference"))
  ;[1 1 1] Comment
  (bind _output_get (set `self.Fpscharacter` fpscharacter))
  (`/Game/Blueprints/FPSCharacter_BP.Inspecteditem` _output_get
    (:`then`)
    (:`else`
      (`self.Inspectitem`))))

(event `Key|LeftMouseButton`
  (params (Key :type "Key Structure"))
  ;[1 1 1] Inspect Item Movement
  (:`Pressed`
    (set `self.Rotate?` true))
  (:`Released`
    (set `self.Rotate?` false)))

(event `InputAxisKey|MouseX`
  (params (AxisValue :type "Float (single-precision)"))
  ;[1 1 1] Inspect Item Movement
  (if (`self.Rotate?`)
    (`self.K2_SetActorRotation` (`KismetMathLibrary.ComposeRotators` (`self.K2_GetActorRotation`) (`KismetMathLibrary.MakeRotator` 0.0 0.0 (* AxisValue 2.0))))))

(event `InputAxisKey|MouseY`
  (params (AxisValue :type "Float (single-precision)"))
  ;[1 1 1] Inspect Item Movement
  (if (`self.Rotate?`)
    (`self.K2_SetActorRotation` (`KismetMathLibrary.ComposeRotators` (`self.K2_GetActorRotation`) (`KismetMathLibrary.MakeRotator` 0.0 (* AxisValue 2.0))))))

(event `Key|RightMouseButton`
  (params (Key :type "Key Structure"))
  (bind (_iteminformation_itemname _iteminformation_itemdescription _iteminformation_itemimage _iteminformation_item _iteminformation_isstackable_) (break `/Game/Blueprints/Inspection/ItemInformation` (`self.ItemInformation`)))
  (bind (_iteminformation_itemname_2 _iteminformation_itemdescription_2 _iteminformation_itemimage_2 _iteminformation_item_2) (break `/Game/Blueprints/Inspection/ItemInformation` (`self.ItemInformation`)))
  (bind (_iteminformation_itemname_3 _iteminformation_itemdescription_3 _iteminformation_itemimage_3 _iteminformation_item_3) (break `/Game/Blueprints/Inspection/ItemInformation` (`self.ItemInformation`)))
  (bind _fpscharacter (`self.Fpscharacter`))
  (bind _inventory (`/Game/Blueprints/FPSCharacter_BP.Inventory` (`self.Fpscharacter`)))
  (bind _inventory_2 (`/Game/Blueprints/FPSCharacter_BP.Inventory` (`self.Fpscharacter`)))
  ;[1 1 1] Add item to players inventory
  (:`Pressed`
    (if (not (`self.FromInventory`))
      (switch `string` (`KismetTextLibrary.Conv_TextToString` _iteminformation_itemname)
        (:`Default`
          (if _iteminformation_isstackable_
            (for _array_element _inventory
              _)
            (if (== (`.Item_10_5B585F634281B3AECF1787A89A286F8B` (break `/Game/Blueprints/Inspection/ItemInformation` _array_element)) _iteminformation_item_3)
              (if (> (`KismetArrayLibrary.Array_Length` _inventory) 0)
                (for (_array_element_2 _array_index) _inventory_2
                  (if (== (`.Item_10_5B585F634281B3AECF1787A89A286F8B` (break `/Game/Blueprints/Inspection/ItemInformation` _array_element_2)) _iteminformation_item_2)
                    (`KismetArrayLibrary.Array_Set` _inventory_2 _array_index (make `/Game/Blueprints/Inspection/ItemInformation` (break `/Game/Blueprints/Inspection/ItemInformation` _array_element_2) (`.ItemDescription_4_310DA46947E17BBAB126E68A97557B58` (break `/Game/Blueprints/Inspection/ItemInformation` _array_element_2)) (`.Itemimage_7_3D8D4B0040A2B8DE268A7FB5B6CB1E41` (break `/Game/Blueprints/Inspection/ItemInformation` _array_element_2)) (`.Item_10_5B585F634281B3AECF1787A89A286F8B` (break `/Game/Blueprints/Inspection/ItemInformation` _array_element_2)) (`.isstackable?_20_3124AB364B21F1FF48C6B1814701FF6B` (break `/Game/Blueprints/Inspection/ItemInformation` _array_element_2)) (+ (`.Number_23_3B51E2014C6A05B3A09AB389937A2F3D` (break `/Game/Blueprints/Inspection/ItemInformation` _array_element_2)) 1)))))
                (else
                  (`KismetArrayLibrary.Array_Add` (`/Game/Blueprints/FPSCharacter_BP.Inventory` (`self.Fpscharacter`)) (`self.ItemInformation`) :!label _label)))
              (else
                (goto _label)))
            (else
              (goto _label))))
        (:`Flashlight`
          (set `/Game/Blueprints/FPSCharacter_BP.Hasflightlight?` true _fpscharacter)
          (`/Game/Blueprints/FPSCharacter_BP.Toggle flashlight` _fpscharacter))
        (:`Blue Battery`
          (`/Engine/EditorBlueprintResources/StandardMacros.IncrementInt` (`/Game/Blueprints/FPSCharacter_BP.boxbatteries` _fpscharacter) :!label _label_2
            (:`  `
              (`/Game/Blueprints/FPSCharacter_BP.CollectedBattery` _fpscharacter)
              (goto _label))))
        (:`Red Battery`
          (goto _label_2))
        (:`Yellow Battery`
          (goto _label_2))
        (:`Green Battery`
          (goto _label_2)))
      (`self.StopInspecting item`)
      (`self.K2_DestroyActor`))))

(fn `Inspectitem`
  (bind _returnvalue (`GameplayStatics.GetPlayerController` 0))
  (bind _returnvalue_2 (`GameplayStatics.GetPlayerCameraManager` 0))
  (bind _staticmesh (`self.StaticMesh`))
  (bind _fpscharacter (`self.Fpscharacter`))
  (bind (_iteminformation_itemname _iteminformation_itemdescription) (break `/Game/Blueprints/Inspection/ItemInformation` (`self.ItemInformation`)))
  (set `self.Itemorginalocation` (`SceneComponent.RelativeLocation` _staticmesh))
  (set `self.Itemorginalrotation` (`SceneComponent.RelativeRotation` _staticmesh))
  (`self.DisableInput` _fpscharacter _returnvalue)
  (`self.EnableInput` _returnvalue)
  (`self.K2_AttachToComponent` (`/Game/Blueprints/FPSCharacter_BP.Item` _fpscharacter) "None" "SnapToTarget" "SnapToTarget" "KeepRelative")
  (`PrimitiveComponent.SetCollisionEnabled` (`self.StaticMesh`) "NoCollision")
  (set `/Game/Blueprints/FPSCharacter_BP.Inspecteditem` self (`self.Fpscharacter`))
  (`self.K2_SetActorLocation` (+ (`PlayerCameraManager.GetCameraLocation` _returnvalue_2) (* (`KismetMathLibrary.GetForwardVector` (`PlayerCameraManager.GetCameraRotation` _returnvalue_2)) (`self.inspectiondistance`))))
  (bind _returnvalue_3 (`|CreateWidget` "/Game/UserInterfaces/Item_WB.Item_WB_C" null _iteminformation_itemname _iteminformation_itemdescription))
  (bind _output_get (set `self.item_UI` _returnvalue_3))
  (`UserWidget.AddToViewport` _output_get 0)
  (if (`self.FromInventory`)
    (`Widget.SetVisibility` (`/Game/UserInterfaces/Item_WB.inventorycontrols` _returnvalue_3) "Visible")
    (else
      (`Widget.SetVisibility` (`/Game/UserInterfaces/Item_WB.inspectcontrols` _returnvalue_3) "Visible"))))

(fn `StopInspecting item`
  (bind _returnvalue (`GameplayStatics.GetPlayerController` 0))
  (bind _item_ui (`self.item_UI`))
  (`self.DisableInput` _returnvalue)
  (`self.EnableInput` (`self.Fpscharacter`) _returnvalue)
  (`self.K2_SetActorRelativeLocation` (`self.Itemorginalocation`))
  (`self.K2_SetActorRelativeRotation` (`self.Itemorginalrotation`))
  (`self.K2_DetachFromActor` "KeepRelative")
  (`PrimitiveComponent.SetCollisionEnabled` (`self.StaticMesh`) "QueryAndPhysics")
  (set `/Game/Blueprints/FPSCharacter_BP.Inspecteditem` null (`self.Fpscharacter`))
  (`/Engine/EditorBlueprintResources/StandardMacros.IsValid` _item_ui
    (:`Is Valid`
      (`Widget.RemoveFromParent` _item_ui))))

(fn `UserConstructionScript`)