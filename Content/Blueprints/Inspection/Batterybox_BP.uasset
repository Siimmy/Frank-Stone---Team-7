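; Battery box that the player interacts with to deposit coloured batteries from their inventory and power a gate lever.
; Each matched battery reveals its mesh, sets its flag and is removed from the inventory, with the loop restarting after each removal.
; Once all four are in, it activates the gate lever and swaps the empty billboard prompt for the full one.
; An older text prompt remains as disconnected, unused logic.
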(event `/Game/Blueprints/Interactinterface.Interact`
  (params (fpscharacter :type "/Game/Blueprints/FPSCharacter_BP Object Reference"))
  (bind _returnvalue (and (`self.Redbattery?`) (`self.Bluebattery?`) (`self.Yellowbattery?`) (`self.Greenbattery?`)))
  ;[1 1 1] Interaction with electrical box batteries
  (`|ExecutionSequence`
    (:`then_1`
      (for (_array_element _array_index) (`/Game/Blueprints/FPSCharacter_BP.Inventory` fpscharacter) :!label _label
        (switch `string` (`KismetTextLibrary.Conv_TextToString` (break `/Game/Blueprints/Inspection/ItemInformation` _array_element))
          (:`Blue Battery`
            (`SceneComponent.SetHiddenInGame` (`self.Bluebattery`) false false)
            (set `self.Bluebattery?` true))
          (:`Red Battery`
            (`SceneComponent.SetHiddenInGame` (`self.Redbattery`) false false)
            (set `self.Redbattery?` true))
          (:`Green Battery`
            (`SceneComponent.SetHiddenInGame` (`self.Greenbattery`) false false)
            (set `self.Greenbattery?` true))
          (:`Yellow Battery`
            (`SceneComponent.SetHiddenInGame` (`self.Yellowbattery`) false false)
            (set `self.Yellowbattery?` true)))
        (`KismetArrayLibrary.Array_RemoveItem` (`/Game/Blueprints/FPSCharacter_BP.Inventory` fpscharacter) (`|GetArrayItem` (`/Game/Blueprints/FPSCharacter_BP.Inventory` fpscharacter) _array_index))
        (goto _label))
      ;;[1 1 1] set gate lever to activated when all batteries collected
      (`|ExecutionSequence`
        (:`then_0`
          (if _returnvalue
            (set `/Game/Blueprints/Interaction/Gatelever_BP.Activated?` true (`self.gatelever`))
            (if _returnvalue
              (set `self.AllBatteriesColected` true)
              (`self.UpdateBillboards`))))))))

(event `UpdateBillboards`
  ;[1 1 1] Billboard Prompt for battery box - change on batteries collected.
  (if (`self.AllBatteriesColected`)
    (`SceneComponent.SetHiddenInGame` (`self.FullBillBoard`) false false)
    (`SceneComponent.SetHiddenInGame` (`self.EmptyBillBoard`) true false)
    (else
      (`SceneComponent.SetHiddenInGame` (`self.FullBillBoard`) true false)
      (`SceneComponent.SetHiddenInGame` (`self.EmptyBillBoard`) false false))))

(fn `UserConstructionScript`)