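; Monster enemy character that roams the navmesh, chases the player on sight and triggers game over on contact.
; It loops AI moves to random nearby points until PawnSensing spots the player, then follows them and fades in chase music.
; A retriggerable delay ends the chase shortly after sightings stop, resuming roaming and fading out the music.
; A capsule hit destroys the player's flashlight, blends the camera to the monster and shows the game-over widget.
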(event `Randomlyroam`
  ;[1 1 1] Randomly roam
  (bind _randomlocation (`NavigationSystemV1.K2_GetRandomLocationInNavigableRadius` (`self.K2_GetActorLocation`) 1000.0 null null :!label _label))
  (`|AIMoveTo` self _randomlocation null
    (:`then`
      (`KismetSystemLibrary.Delay` 4.0 :!label _label_2)
      (if (not (`self.seesplayer?`))
        (`self.Randomlyroam`)))
    (:`OnSuccess`
      (goto _label_2))
    (:`OnFail`
      (`KismetSystemLibrary.PrintString` "failed to find path"))))

(event `self.ReceiveBeginPlay`
  ;[1 1 1] Randomly roam
  (set `CharacterMovementComponent.MaxWalkSpeed` (`self.Monster speed`) (`self.CharacterMovement`))
  (goto _label))

(event `self.PawnSensing.OnSeePawn`
  (params (Pawn :type "Pawn Object Reference"))
  (bind _returnvalue (`GameplayStatics.GetPlayerCharacter` 0))
  ;[1 1 1] When monster sees player
  (if (== Pawn _returnvalue)
    (`|ExecutionSequence`
      (:`then_0`
        (set `self.seesplayer?` true)
        (`|AIMoveTo` self (0.0 0.0 0.0) _returnvalue
          (:`then`
            (`self.chasesequence`
              (:`then`)
              (:`else`
                (bind _returnvalue_2 (`GameplayStatics.SpawnSound2D` null 1.0 1.0 0.0 null))
                (bind _output_get (set `self.chasesequence` _returnvalue_2))
                (`AudioComponent.FadeIn` _output_get 1.0 1.0 0.0 "Linear"))))
          (:`OnFail`
            (`KismetSystemLibrary.PrintString` "failed - seeing player"))))
      (:`then_1`
        (`KismetSystemLibrary.RetriggerableDelay` 1.5)
        (set `self.seesplayer?` false)
        (`self.Randomlyroam`)
        (bind _chasesequence (`self.chasesequence`)
          (:`then`
            (`AudioComponent.FadeOut` _chasesequence 1.0 0.0 "Linear")
            (`KismetSystemLibrary.Delay` 1.0)
            (set `self.chasesequence` null))
          (:`else`))))))

(event `self.CapsuleComponent.OnComponentHit`
  (params (HitComponent :type "PrimitiveComponent Object Reference") (OtherActor :type "Actor Object Reference") (OtherComp :type "PrimitiveComponent Object Reference") (NormalImpulse :type "Vector Structure") (Hit :type "HitResult Structure (by ref)"))
  ;[1 1 1] Kill player when he hits monster
  (bind _asfpscharacter_bp (cast `/Game/Blueprints/FPSCharacter_BP` OtherActor))
  (`/Engine/EditorBlueprintResources/StandardMacros.DoOnce` false
    (:`Completed`
      (`self.K2_DestroyActor` (`/Game/Blueprints/FPSCharacter_BP.flashlighref` _asfpscharacter_bp))
      (`PlayerController.SetViewTargetWithBlend` (`GameplayStatics.GetPlayerController` 0) self 0.3 "VTBlend_Linear" 0.0 false)
      (bind _returnvalue (`|CreateWidget` "/Game/UserInterfaces/Gameover_WB.Gameover_WB_C"))
      (`UserWidget.AddToViewport` _returnvalue 0))))

(fn `UserConstructionScript`)