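; Enemy character that ends the game when its capsule hits the player.
; The first hit destroys the player's flashlight, blends the camera to the enemy and shows the game over widget.
; A battery collection event sets its walk speed to MonsterSpeed.
; Despite the pathfinding name, MoveNPC, BeginPlay and ResetAistate are empty, and audio setup, run-away, stop and montage logic are unconnected.
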(event `self.CapsuleComponent.OnComponentHit`
  (params (HitComponent :type "PrimitiveComponent Object Reference") (OtherActor :type "Actor Object Reference") (OtherComp :type "PrimitiveComponent Object Reference") (NormalImpulse :type "Vector Structure") (Hit :type "HitResult Structure (by ref)"))
  ;[1 1 1] Kill player when he hits
  (bind _asfpscharacter_bp (cast `/Game/Blueprints/FPSCharacter_BP` OtherActor))
  (`/Engine/EditorBlueprintResources/StandardMacros.DoOnce` false
    (:`Completed`
      (`self.K2_DestroyActor` (`/Game/Blueprints/FPSCharacter_BP.flashlighref` _asfpscharacter_bp))
      (`PlayerController.SetViewTargetWithBlend` (`GameplayStatics.GetPlayerController` 0) self 0.3 "VTBlend_Linear" 0.0 false)
      (bind _returnvalue (`|CreateWidget` "/Game/UserInterfaces/Gameover_WB.Gameover_WB_C"))
      (`UserWidget.AddToViewport` _returnvalue 0))))

(event `Battery collected`
  ;[1 1 1] When battery is collected
  (set `CharacterMovementComponent.MaxWalkSpeed` (`self.MonsterSpeed`) (`self.CharacterMovement`)))

(event `self.ReceiveBeginPlay`
  ;[1 1 1] Create Audio ref
)

(event `ResetAistate`)

(fn `MoveNPC`)

(fn `UserConstructionScript`)