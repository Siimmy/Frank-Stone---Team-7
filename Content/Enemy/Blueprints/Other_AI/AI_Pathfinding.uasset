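; AI controller for an enemy that runs the BT_AIPathfinding behavior tree and reacts to seeing the player.
; Sight perception updates set the Blackboard's TargetActor to the player, or clear it when sight is lost, and cache the player character reference.
; A recursive RunAway function picks random reachable points away from the player but casts the player's controller to AIController.
; RunAway and the last-known-location update are disconnected from live execution.
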(event `self.ReceiveBeginPlay`
  (`self.RunBehaviorTree` "/Game/Enemy/Blueprints/Other_AI/BT_AIPathfinding.BT_AIPathfinding"))

(event `self.AIPerception.OnTargetPerceptionUpdated`
  (params (Actor :type "Actor Object Reference") (Stimulus :type "AIStimulus Structure"))
  (`self.HandleSightSense` Actor Stimulus))

(fn `HandleSightSense`
  (params (Actor :type "Actor Object Reference") (Stimulus :type "AIStimulus Structure"))
  (bind (_stimulus_age _stimulus_expirationage _stimulus_strength _stimulus_stimuluslocation _stimulus_receiverlocation _stimulus_tag _stimulus_bsuccessfullysensed) (break `AIStimulus` (`local.Stimulus`)))
  (bind _returnvalue (`AIPerceptionSystem.GetSenseClassForStimulus` Stimulus))
  ;[1 1 1] check to see if player
  (if (== _returnvalue "/Script/AIModule.AISense_Sight")
    ;[1 1 1] if yes set value of player as object value
    (if (== (`local.Actor`) (`GameplayStatics.GetPlayerCharacter` 0))
      (`BlackboardComponent.SetValueAsObject` (`self.Blackboard`) "TargetActor" (`KismetMathLibrary.SelectObject` (`GameplayStatics.GetPlayerCharacter` 0) null _stimulus_bsuccessfullysensed))
      ;[1 1 1] when loses sight put into vector and use as last knwon location
      (if _stimulus_bsuccessfullysensed
        ;[1 1 1] Create ref to character
        (bind _asfpscharacter_bp (cast `/Game/Blueprints/FPSCharacter_BP` (`GameplayStatics.GetPlayerCharacter` 0)))
        (set `self.Character ref` _asfpscharacter_bp))
      (else
        (return)))
    (else
      (return))))

(fn `Run Away`
  (bind _returnvalue (`self.K2_GetActorLocation`))
  (`KismetSystemLibrary.PrintString` "runawaytriggered")
  (bind _asaicontroller (cast `AIController` (`Pawn.GetController` (`self.Character ref`))))
  (`self.MoveToLocation` _asaicontroller (`NavigationSystemV1.K2_GetRandomReachablePointInRadius` (`KismetMathLibrary.MakeVector` (.x (+ _returnvalue (* (`KismetMathLibrary.GetForwardVector` (`KismetMathLibrary.FindLookAtRotation` _returnvalue (`self.K2_GetActorLocation` (`self.Character ref`)))) -500.0))) (.y (+ _returnvalue (* (`KismetMathLibrary.GetForwardVector` (`KismetMathLibrary.FindLookAtRotation` _returnvalue (`self.K2_GetActorLocation` (`self.Character ref`)))) -500.0))) (.z _returnvalue)) 500.0 null null) 5.0 true true false true null true)
  (`self.Run Away`))

(fn `UserConstructionScript`)