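; AI_Enemy_BP is a monster that roams, hunts the player and ends the game on contact.
; Pawn sensing starts a chase with audio; a retriggerable delay clears sight, letting Tick fade audio and resume random roaming.
; A capsule hit destroys the player's flashlight, blends the view to the monster and shows game over.
; A looping RunAway flee starts at BeginPlay, and battery collection sets walk speed to MonsterSpeed.
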(event `self.CapsuleComponent.OnComponentHit`
  (params (HitComponent :type "PrimitiveComponent Object Reference") (OtherActor :type "Actor Object Reference") (OtherComp :type "PrimitiveComponent Object Reference") (NormalImpulse :type "Vector Structure") (Hit :type "HitResult Structure (by ref)"))
  ;[1 1 1] Kill player when he hits monster
  (bind _asfpscharacter_bp (cast `/Game/Blueprints/FPSCharacter_BP` OtherActor))
  (`/Engine/EditorBlueprintResources/StandardMacros.DoOnce` false
    (:`Completed`
      (`self.K2_DestroyActor` (`/Game/Blueprints/FPSCharacter_BP.flashlighref` _asfpscharacter_bp))
      (`PlayerController.SetViewTargetWithBlend` (`GameplayStatics.GetPlayerController` 0) self 0.3 "VTBlend_Linear" 0.0 false)
      (bind _returnvalue (`|CreateWidget` "/Game/UserInterfaces/Gameover_WB.Gameover_WB_C"))
      (`UserWidget.AddToViewport` _returnvalue 0))))

(event `Battery collected`
  ;[1 1 1] When battery is collected
  (set `CharacterMovementComponent.MaxWalkSpeed` (`self.MonsterSpeed`) (`self.CharacterMovement`)))

(event `self.PawnSensing.OnSeePawn`
  (params (Pawn :type "Pawn Object Reference"))
  ;[1 1 1] Pawn sensing - move to player - and random roam within radius
  (bind _asfpscharacter_bp (cast `/Game/Blueprints/FPSCharacter_BP` Pawn))
  (`|ExecutionSequence`
    (:`then_0`
      (set `self.Can see Enemy?` true)
      (set `self.isChasing?` true)
      (`|AIMoveTo` self (0.0 0.0 0.0) _asfpscharacter_bp
        (:`then`
          (`/Engine/EditorBlueprintResources/StandardMacros.DoOnce` false :!label _label
            (:`Completed`
              (`AudioComponent.Play` (`self.Audio`) 0.0))))))
    (:`then_1`
      (`KismetSystemLibrary.RetriggerableDelay` 0.6)
      (set `self.Can see Enemy?` false))))

(event `self.ReceiveTick`
  (params (DeltaSeconds :type "Float (single-precision)"))
  ;[1 1 1] Pawn sensing - move to player - and random roam within radius
  (`|ExecutionSequence`
    (:`then_0`
      (if (not (`self.Can see Enemy?`))
        (`KismetSystemLibrary.Delay` 0.1)
        (if (not (`self.Can see Enemy?`))
          (`AudioComponent.FadeOut` (`self.Audio`) 5.0 0.0 "Linear")
          (set `self.isChasing?` false)
          (goto _label :!via `Reset`))))
    (:`then_1`
      (if (not (`self.isChasing?`))
        (`KismetSystemLibrary.Delay` (`KismetMathLibrary.RandomFloatInRange` 2.0 3.0))
        (`|AIMoveTo` self (`NavigationSystemV1.K2_GetRandomReachablePointInRadius` (`self.K2_GetActorLocation`) 2000.0 null null) null)))))

(event `self.ReceiveBeginPlay`
  ;[1 1 1] Create Audio ref
  (`|ExecutionSequence`
    (:`then_0`
      (bind _returnvalue (`AddComponent|NODE_AddAudioComponent-0`))
      (`AudioComponent.Stop` _returnvalue)
      (set `self.Audio` _returnvalue))
    (:`then_1`
      ;[1 1 1] Create ref to character
      (bind _asfpscharacter_bp (cast `/Game/Blueprints/FPSCharacter_BP` (`GameplayStatics.GetPlayerCharacter` 0)))
      (set `self.Charcter ref` _asfpscharacter_bp)
      (`self.RunAway`))))

(event `RunAway`
  (bind _returnvalue (`self.K2_GetActorLocation`))
  ;[1 1 1] Run away to within radius  - event called when collision with torch component
  (`|AIMoveTo` self (`NavigationSystemV1.K2_GetRandomReachablePointInRadius` (`KismetMathLibrary.MakeVector` (.x (+ _returnvalue (* (`KismetMathLibrary.GetForwardVector` (`KismetMathLibrary.FindLookAtRotation` _returnvalue (`self.K2_GetActorLocation` (`self.Charcter ref`)))) -500.0))) (.y (+ _returnvalue (* (`KismetMathLibrary.GetForwardVector` (`KismetMathLibrary.FindLookAtRotation` _returnvalue (`self.K2_GetActorLocation` (`self.Charcter ref`)))) -500.0))) (.z _returnvalue)) 500.0 null null) null
    (:`OnSuccess`
      _)
    (:`OnFail`
      _))
  (`self.RunAway`))

(event `ResetAistate`
  (`MovementComponent.StopMovementImmediately` (`self.CharacterMovement`)))

(fn `MoveNPC`)

(fn `UserConstructionScript`)